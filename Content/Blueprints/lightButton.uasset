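; Pressable light button component that changes a target lamp when left-clicked under the screen centre at close range.
; Tick projects the viewport-centre ray to the button's distance and requires the lamp to be lit.
; An On flag and paired DoOnce gates select LightControl or its negation for LightChangeLamp.
; Presses call CallLightChange and briefly teleport the owner along MoveDir from its parent Cube_Blueprint.
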(event Custom|mousePos)

(event EventBeginPlay
  (bind _returnvalue (Game|GetPlayerController 0))
  (Variables|/Script/Engine.PlayerController|SetbEnableMouseOverEvents _returnvalue true)
  (Variables|/Script/Engine.PlayerController|SetbEnableClickEvents _returnvalue true)
  (bind _ascube_blueprint (Utilities|Casting|CastToCube_Blueprint (Components|GetOwner (Transformation|GetAttachParent (VehicleSound|GetRootComponent (Components|GetOwner))))))
  (Variables|Default|SetmoveDir (Variables|/Game/Blueprints/Cube_Blueprint.Cube_Blueprint_C|GetmoveDir _ascube_blueprint)))

(event EventTick
  (params (DeltaSeconds :type Float%20%28single-precision%29))
  (bind _returnvalue (Components|GetOwner))
  (bind _returnvalue_2 (Game|GetPlayerController 0))
  (bind _returnvalue_3 (Viewport|GetViewportSize))
  (bind _self self)
  (bind _targetlight (Variables|Default|GettargetLight))
  (bind _movedir (Variables|Default|GetmoveDir))
  (bind _returnvalue_4 (Transformation|GetActorLocation _returnvalue))
  (bind _returnvalue_5 (Components|GetOwner _self))
  (bind _returnvalue_6 (Transformation|GetActorRotation _returnvalue))
  (bind (_x _y) (Math|Vector2D|BreakVector2D _returnvalue_3))
  (bind _returnvalue_7 (Transformation|GetActorLocation _returnvalue_5))
  (bind _returnvalue_8 (/ _x 2.0))
  (bind _returnvalue_9 (/ _y 2.0))
  (bind (_worldlocation _worlddirection) (Class|PlayerController|DeprojectScreenPositiontoWorld _returnvalue_2 _returnvalue_8 _returnvalue_9))
  (bind _returnvalue_10 (- _worldlocation _returnvalue_7))
  (bind _returnvalue_11 (Math|Vector|VectorLength _returnvalue_10))
  (CallFunction|MousePos)
  (if (Math|Boolean|ANDBoolean (== (Class|PlayerController|GetInputAnalogKeyState (Game|GetPlayerController 0) "LeftMouseButton") 1.0) (< (Math|Vector|VectorLength (- _returnvalue_7 (+ (* _worlddirection _returnvalue_11) _worldlocation))) 3e+01) (> (Variables|/Script/Engine.LightComponentBase|GetIntensity (Variables|/Game/Blueprints/lamp_Blueprint.lamp_Blueprint_C|GetSpotLight (Variables|Default|GettargetLight))) 0.0) (< _returnvalue_11 3e+02))
    (if (Variables|Default|Geton)
      (Utilities|FlowControl|DoOnce false :!label _label
        (:Completed
          (Default|LightChangeLamp _targetlight (Variables|Default|GetlightControl))
          (Utilities|FlowControl|Sequence
            (:then_0
              (goto _label_2 Reset))
            (:then_1
              _))))
      (else
        (Utilities|FlowControl|DoOnce false :!label _label_2
          (:Completed
            (Default|LightChangeLamp _targetlight (* (Variables|Default|GetlightControl) -1))
            (Utilities|FlowControl|Sequence
              (:then_0
                (goto _label Reset))
              (:then_1
                _))))))
    (Transformation|Teleport _returnvalue (+ _returnvalue_4 (* _movedir -5)) _returnvalue_6)
    (Default|CallLightChange (Variables|Default|GetlightControl))
    (Utilities|FlowControl|Delay 1.0)
    (Transformation|Teleport _returnvalue (+ _returnvalue_4 (* _movedir 5)) _returnvalue_6)
    (Variables|Default|Seton (not (Variables|Default|Geton)))))