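; Indicator light Blueprint that shows a mix of red, green and blue channels as one of eight sphere materials.
; On BeginPlay it collects LightButton components from actors attached to a target and binds their light-change events.
; Each event toggles the channels whose delta component equals one, using XOR.
; Tick packs the three booleans into a bitmask and switches the sphere's material accordingly.
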(event Custom|changeLightColor
  (params (deltaColor :type Vector))
  (bind (_x _y _z) (Math|Vector|BreakVector deltaColor))
  (Variables|Default|Setred (Class|KismetMathLibrary|XORBoolean (Variables|Default|Getred) (== _x 1.0)))
  (Variables|Default|Setgreen (Class|KismetMathLibrary|XORBoolean (Variables|Default|Getgreen) (== _y 1.0)))
  (Variables|Default|Setblue (Class|KismetMathLibrary|XORBoolean (Variables|Default|Getblue) (== _z 1.0))))

(event EventTick
  (params (DeltaSeconds :type Float%20%28single-precision%29))
  (switch int (+ (Math|Conversions|ToInteger(Boolean) (Variables|Default|Getred)) (* (Math|Conversions|ToInteger(Boolean) (Variables|Default|Getgreen)) 2) (* (Math|Conversions|ToInteger(Boolean) (Variables|Default|Getblue)) 4))
    (:0
      (Rendering|Material|SetMaterial (Variables|Default|GetSphere) 0 "/Game/StarterContent/Blueprints/Assets/M_LightStage_Skybox_Black.M_LightStage_Skybox_Black"))
    (:1
      (Rendering|Material|SetMaterial (Variables|Default|GetSphere) 0 "/Game/Materials/redBlock.redBlock"))
    (:2
      (Rendering|Material|SetMaterial (Variables|Default|GetSphere) 0 "/Game/Materials/greenBlock.greenBlock"))
    (:3
      (Rendering|Material|SetMaterial (Variables|Default|GetSphere) 0 "/Game/Materials/yellowBlock.yellowBlock"))
    (:4
      (Rendering|Material|SetMaterial (Variables|Default|GetSphere) 0 "/Game/Materials/blueBlock.blueBlock"))
    (:5
      (Rendering|Material|SetMaterial (Variables|Default|GetSphere) 0 "/Game/Materials/magentaBlock.magentaBlock"))
    (:6
      (Rendering|Material|SetMaterial (Variables|Default|GetSphere) 0 "/Game/Materials/cyanBlock.cyanBlock"))
    (:7
      (Rendering|Material|SetMaterial (Variables|Default|GetSphere) 0 "/Game/StarterContent/Materials/M_Basic_Wall.M_Basic_Wall"))))

(event EventBeginPlay
  (for _array_element (Actor|GetAttachedActors (Variables|Default|Gettarget))
    (Utilities|Array|Add (Variables|Default|Getbuttons) (Utilities|Array|Get(acopy) (Actor|GetComponentsByClass _array_element "/Game/Blueprints/lightButton.lightButton_C")))
    (EventDispatchers|BindEventtoLightChange (Utilities|Array|Get(acopy) (Actor|GetComponentsByClass _array_element "/Game/Blueprints/lightButton.lightButton_C")) (delegate Custom|changeLightColor))))

(fn ConstructionScript)