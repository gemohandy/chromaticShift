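; Lamp Blueprint that controls a spotlight whose color and brightness other code can change.
; BeginPlay resets the SpotLight color to white, and the lightUp event sets it to a fixed, very high intensity.
; LightChangeLamp adds a vector offset to the current RGB color, clamping each channel at zero with no upper limit and keeping alpha.
; The returnBright graph is empty.
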(event Custom|lightUp
  (Rendering|Components|Light|SetIntensity (Variables|Default|GetSpotLight) 1e+05))

(event Collision|EventActorBeginOverlap
  (params (OtherActor :type Actor%20Object%20Reference)))

(event EventTick
  (params (DeltaSeconds :type Float%20%28single-precision%29)))

(event EventBeginPlay
  (Rendering|Components|Light|SetLightColor (Variables|Default|GetSpotLight) (Math|Color|MakeColor 1.0 1.0 1.0) true))

(fn ConstructionScript)

(fn LightChangeLamp
  (params (color :type Vector))
  (bind _spotlight (Variables|Default|GetSpotLight))
  (bind _returnvalue (Rendering|Components|Light|GetLightColor _spotlight))
  (bind (_r _g _b _a) (Math|Color|BreakColor _returnvalue))
  (bind _returnvalue_2 (Math|Vector|MakeVector _r _g _b))
  (bind _returnvalue_3 (+ color _returnvalue_2))
  (bind (_x _y _z) (Math|Vector|BreakVector _returnvalue_3))
  (Rendering|Components|Light|SetLightColor (Variables|Default|GetSpotLight) (Math|Color|MakeColor (Math|Float|Max(Float) _x 0.0) (Math|Float|Max(Float) _y 0.0) (Math|Float|Max(Float) _z 0.0) _a) true))