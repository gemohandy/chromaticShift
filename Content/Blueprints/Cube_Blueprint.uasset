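; Cube Blueprint that performs a one-time animated turn, rolling and shifting its static mesh when the turn event fires.
; A HasTurned flag, cleared on BeginPlay, blocks repeat turns.
; A custom delayFor macro loops with a short Delay between iterations.
; Each iteration offsets world location by MoveDir and decrements roll, totalling roughly a quarter turn without sweep.
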(event Custom|turn
  (bind _staticmeshcomponent (Variables|Debug|GetStaticMeshComponent))
  (bind _returnvalue (Transformation|GetWorldTransform _staticmeshcomponent))
  (bind (_location _rotation _scale) (Math|Transform|BreakTransform _returnvalue))
  (bind (_roll _pitch _yaw) (Math|Rotator|BreakRotator _rotation))
  (if (not (Variables|Default|GethasTurned))
    (Variables|Default|SethasTurned true)
    (Utilities|Delayfor 0 50 0.0005
      (:loop%20body
        (Transformation|SetWorldTransform (Variables|Debug|GetStaticMeshComponent) (Math|Transform|MakeTransform (+ _location (Variables|Default|GetmoveDir)) (Math|Rotator|MakeRotator (+ _roll -1.8) _pitch _yaw) _scale) false false)))))

(event EventBeginPlay
  (Variables|Default|SethasTurned false))

(fn ConstructionScript)