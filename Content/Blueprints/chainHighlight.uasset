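; Highlightable actor that lights up when screen center points near it at close range, and triggers its targets on left click.
; Each Tick deprojects screen center for the aim test, attaching Lit emitters while aimed with a child-count cap, otherwise destroying all mesh child components.
; A click calls CallActivator on every Targets entry, then raises the actor through a delayed-loop macro whose body re-enters the loop after each step.
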(event EventBeginPlay
  (bind _returnvalue (Game|GetPlayerController 0))
  (Variables|/Script/Engine.PlayerController|SetbEnableMouseOverEvents _returnvalue true)
  (Variables|/Script/Engine.PlayerController|SetbEnableClickEvents _returnvalue true))

(event Collision|EventActorBeginOverlap
  (params (OtherActor :type Actor%20Object%20Reference)))

(event EventTick
  (params (DeltaSeconds :type Float%20%28single-precision%29))
  (bind _returnvalue (Game|GetPlayerController 0))
  (bind _returnvalue_2 (Viewport|GetViewportSize))
  (bind _self self)
  (bind _staticmeshcomponent (Variables|Debug|GetStaticMeshComponent))
  (bind _children (Components|GetChildrenComponents _staticmeshcomponent true))
  (bind _returnvalue_3 (Transformation|GetActorLocation _self))
  (bind (_x _y) (Math|Vector2D|BreakVector2D _returnvalue_2))
  (bind _returnvalue_4 (/ _x 2.0))
  (bind _returnvalue_5 (/ _y 2.0))
  (bind (_worldlocation _worlddirection) (Class|PlayerController|DeprojectScreenPositiontoWorld _returnvalue _returnvalue_4 _returnvalue_5))
  (bind _returnvalue_6 (- _worldlocation _returnvalue_3))
  (bind _returnvalue_7 (Math|Vector|VectorLength _returnvalue_6))
  (if (Math|Boolean|ANDBoolean (> 25 (Utilities|Array|Length _children)) (< (Math|Vector|VectorLength (- _returnvalue_3 (+ (* _worlddirection _returnvalue_7) _worldlocation))) 5e+01) (< _returnvalue_7 4e+02))
    (Effects|SpawnEmitterAttached "/Game/StarterContent/Particles/lit.lit" (Variables|Debug|GetStaticMeshComponent) "None")
    (if (== (Class|PlayerController|GetInputAnalogKeyState (Game|GetPlayerController 0) "LeftMouseButton") 1.0)
      (for _array_element (Variables|Default|Gettargets)
        (Default|CallActivator _array_element))
      (Utilities|ForwithDelay 0 500 2e-05 :!label _label
        (:run
          (Transformation|SetActorLocation (+ (Transformation|GetActorLocation) "0,0.000000,1.000000") false false)
          (Utilities|FlowControl|Delay 3e-05)
          (goto _label))))
    (else
      (for _array_element_2 _children
        (Components|DestroyComponent _array_element_2)))))

(fn ConstructionScript)