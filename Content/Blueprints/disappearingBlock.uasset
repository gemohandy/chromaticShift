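; disappearingBlock turns its owning actor's collision on or off based on a lamp's light color and which color channels the player can see.
; On BeginPlay it finds and stores the player-controlled FirstPersonCharacter.
; Each Tick it compares RelevantLamp's spotlight to AllowedColor per RGB channel, skipping channels the player cannot see.
; Collision is disabled when no visible channel exceeds its limit and enabled otherwise, with no change to visibility.
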(event EventTick
  (params (DeltaSeconds :type Float%20%28single-precision%29))
  (bind _returnvalue (Components|GetOwner))
  (bind _player (Variables|Default|Getplayer))
  (bind _relevantlamp (Variables|Default|GetrelevantLamp))
  (bind _allowedcolor (Variables|Default|GetallowedColor))
  (bind (_r _g _b) (Math|Color|BreakColor _allowedcolor))
  (bind _spotlight (Variables|/Game/Blueprints/lamp_Blueprint.lamp_Blueprint_C|GetSpotLight _relevantlamp))
  (bind _returnvalue_2 (Rendering|Components|Light|GetLightColor _spotlight))
  (bind (_r_2 _g_2 _b_2) (Math|Color|BreakColor _returnvalue_2))
  (if (Math|Boolean|ANDBoolean (or (<= _r_2 _r) (not (Variables|/Game/FirstPersonBP/Blueprints/FirstPersonCharacter.FirstPersonCharacter_C|GetseeRed _player))) (or (<= _g_2 _g) (not (Variables|/Game/FirstPersonBP/Blueprints/FirstPersonCharacter.FirstPersonCharacter_C|GetseeGreen _player))) (or (<= _b_2 _b) (not (Variables|/Game/FirstPersonBP/Blueprints/FirstPersonCharacter.FirstPersonCharacter_C|GetseeBlue _player))))
    (Collision|SetActorEnableCollision _returnvalue false)
    (else
      (Collision|SetActorEnableCollision _returnvalue true))))

(event EventBeginPlay
  (bind _outactors (Actor|GetAllActorsOfClass "/Game/FirstPersonBP/Blueprints/FirstPersonCharacter.FirstPersonCharacter_C"))
  (for _array_element _outactors
    (if (Pawn|IsPlayerControlled _array_element)
      (Variables|Default|Setplayer _array_element))))